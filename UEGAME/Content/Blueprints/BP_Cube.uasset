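; BP_Cube is an actor that colors its mesh black and repositions itself once at BeginPlay.
; A dynamic material instance on StaticMesh sets the Color parameter, then Case3 rotates the actor to a fixed yaw and offsets it along that heading.
; Case1 (diagonal offset only) and Case2 (world X offset plus yaw) are alternative transform examples that nothing in this file calls.
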(event Custom|Case1
  ;[0.06679 0.4843 1] Case1
  (Transformation|SetActorLocation (+ (Transformation|GetActorLocation) (Math|Vector|MakeVector 1e+02 1e+02 0.0)) false false))

(event Custom|Case2
  ;[1 1 1] Case2
  (Transformation|SetActorLocationAndRotation (+ (Transformation|GetActorLocation) (Math|Vector|MakeVector 1e+02 0.0 0.0)) (Math|Rotator|MakeRotator 0.0 0.0 45.0)))

(event Custom|Case3
  ;[1 1 1] Case3
  (Transformation|SetActorLocationAndRotation (+ (Transformation|GetActorLocation) (* (Class|KismetMathLibrary|VectorNormal2D (Math|Vector|GetForwardVector (Math|Rotator|MakeRotator 0.0 0.0 45.0)) 0.0001) 1e+02)) (Math|Rotator|MakeRotator 0.0 0.0 45.0)))

(event EventBeginPlay
  (Utilities|FlowControl|Sequence
    (:then_0
      (bind _returnvalue (Rendering|Material|CreateDynamicMaterialInstance (Variables|Default|GetStaticMesh) 0 0 "None" :!class /Script/Engine.PrimitiveComponent))
      (bind _output_get (Variables|Default|SetMaterial _returnvalue))
      (Rendering|Material|SetMaterial (Variables|Default|GetStaticMesh) 0 _output_get)
      (Rendering|Material|SetVectorParameterValue (Variables|Default|GetMaterial) "Color" "(R=0.000000,G=0.000000,B=0.000000,A=1.000000)" :!class /Script/Engine.MaterialInstanceDynamic))
    (:then_1
      (CallFunction|Case3))))

(fn ConstructionScript)